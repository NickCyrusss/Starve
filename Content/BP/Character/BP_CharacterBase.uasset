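; Base character Blueprint that lets a character interact with nearby actors when the Interactive input is pressed.
; The press is passed through a Server Attack event to a Client Attack event, which does the detection.
; A sphere overlap around the character, filtered to one object type, sends InteractiveMessage with the character as argument to each actor found.
; A debug sphere and printed actor names show the results.
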(event Custom|Server_Attack
  ;[1 1 1] E
  (CallFunction|ClientAttack))

(event Custom|Client_Attack
  (bind _returnvalue (Transformation|GetActorLocation))
  ;[1 1 1] E
  (bind (_outactors _returnvalue_2) (Collision|SphereOverlapActors _returnvalue 1.2e+02 (Utilities|Array|MakeArray "ObjectTypeQuery7") 0))
  (Rendering|Debug|DrawDebugSphere _returnvalue 1.2e+02 32 "(R=0.000000,G=8.089378,B=30.000000,A=1.000000)" 0.5 1.0)
  (if _returnvalue_2
    (for _array_element _outactors
      (Class|IItem|Interactive(Message) _array_element self)
      (Development|PrintString (Utilities|GetDisplayName _array_element)))))

(event Input|ActionEvents|InputActionInteractive
  (params (Key :type Key%20Structure))
  ;[1 1 1] E
  (:Pressed
    (CallFunction|ServerAttack)))

(fn ConstructionScript)