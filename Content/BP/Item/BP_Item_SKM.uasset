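; BP_Item_SKM is an item Blueprint that displays an item as an animated skeletal mesh.
; Its construction script runs the parent script, then, for a non-negative ItemData ID flagged as skeletal, applies that data's mesh and overrides its animation.
; Valid IDs without the skeletal flag show a "Not SKM!" error.
; The event graph holds only disabled placeholder events, so all of the Blueprint's own logic runs at construction.
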(event EventBeginPlay
  (|CallParentFunction) ; This node is disabled and will not be called.\nDrag off pins to build functionality.
)

(event Collision|EventActorBeginOverlap
  (params (OtherActor :type Actor%20Object%20Reference))
  (|CallParentFunction OtherActor) ; This node is disabled and will not be called.\nDrag off pins to build functionality.
)

(event EventTick
  (params (DeltaSeconds :type Float%20%28single-precision%29))
  (|CallParentFunction DeltaSeconds) ; This node is disabled and will not be called.\nDrag off pins to build functionality.
)

(fn ConstructionScript
  (bind _itemdata (Variables|Default|GetItemData))
  (bind _skeletalmesh (Variables|Default|GetSkeletalMesh))
  (bind (_id _name _description _icon _sm _isskm _skm _anim) (Utilities|Struct|BreakST_Item _itemdata))
  (|CallParentFunction)
  (if (>= _id 0)
    (if _isskm
      (Class|SkinnedMeshComponent|SetSkeletalMesh _skeletalmesh _skm true)
      (Components|Animation|OverrideAnimationData _skeletalmesh _anim true true 0.0 1.0)
      (else
        (CallFunction|ShowErrorMessage "Not SKM!")))))