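; BP_Item_SM is an item actor that displays a static mesh taken from its ItemData.
; When ItemData has a non-negative ID, the construction script assigns its mesh to the StaticMesh component, or shows a "Not SM" error if the data is flagged as skeletal.
; The Interactive event is an empty stub, and the graph has no active runtime logic.
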(event EventBeginPlay
  (|CallParentFunction) ; This node is disabled and will not be called.\nDrag off pins to build functionality.
)

(event Collision|EventActorBeginOverlap
  (params (OtherActor :type Actor%20Object%20Reference))
  (|CallParentFunction OtherActor) ; This node is disabled and will not be called.\nDrag off pins to build functionality.
)

(event EventTick
  (params (DeltaSeconds :type Float%20%28single-precision%29))
  (|CallParentFunction DeltaSeconds) ; This node is disabled and will not be called.\nDrag off pins to build functionality.
)

(event EventInteractive
  (params (Operater :type BP%20Character%20Base%20Object%20Reference)))

(fn ConstructionScript
  (bind _itemdata (Variables|Default|GetItemData))
  (bind (_id _name _description _icon _sm _isskm) (Utilities|Struct|BreakST_Item _itemdata))
  (|CallParentFunction)
  (if (>= _id 0)
    (if _isskm
      (CallFunction|ShowErrorMessage "Not SM")
      (else
        (Components|StaticMesh|SetStaticMesh (Variables|Default|GetStaticMesh) _sm)))))